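; BP_Ball is a ball pawn that AI-moves to a Destination actor, then passes to player control.
; BeginPlay points the first player controller's view at Camera and calls ActivatePhysics.
; Tick issues AIMoveTo until it succeeds and sets Found.
; Once Found is true, every tick possesses the ball with that controller and repeats the view-target and physics calls.
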(event `self.ReceiveBeginPlay`
  (`PlayerController.SetViewTargetWithBlend` (`GameplayStatics.GetPlayerController` 0) (`self.camera`) 0.0 "VTBlend_Linear" 0.0 false :!label _label)
  (`self.ActivatePhysics`))

(event `self.ReceiveTick`
  (params (DeltaSeconds :type "Float (single-precision)"))
  (if (`self.found`)
    (`Controller.Possess` (`GameplayStatics.GetPlayerController` 0) self)
    (goto _label)
    (else
      (`|AIMoveTo` self (0.0 0.0 0.0) (`self.Destination`)
        (:`OnSuccess`
          (set `self.found` true))))))

(fn `UserConstructionScript`)